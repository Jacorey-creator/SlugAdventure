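; Menu game mode that tracks connected BP_Menu_Controller players and keeps lobby player names in sync.
; On the Lobby level, each new player is added to the connected list and told to create its lobby menu and run initial setup.
; Logout removes the controller and triggers UpdateLobby, which, when flagged for names, rebuilds the profile array from all controllers and sends it back to each one.
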(event `self.K2_OnLogout`
  (params (ExitingController :type "Controller Object Reference"))
  (bind _asbp_menu_controller (cast `/Game/GAME/Framework/BP_Menu_Controller` ExitingController))
  (`KismetArrayLibrary.Array_RemoveItem` (`self.AllConnectedPlayers`) _asbp_menu_controller)
  (`self.UpdateLobby` true))

(event `self.HandleStartingNewPlayer`
  (params (NewPlayer :type "PlayerController Object Reference"))
  (bind _returnvalue (`GameplayStatics.GetCurrentLevelName` true))
  (switch `string` _returnvalue
    (:`LobbyLevel`
      (bind _asbp_menu_controller (cast `/Game/GAME/Framework/BP_Menu_Controller` NewPlayer))
      (`KismetArrayLibrary.Array_Add` (`self.AllConnectedPlayers`) _asbp_menu_controller)
      (`/Game/GAME/Framework/BP_Menu_Controller.CreateLobbyMenu` _asbp_menu_controller)
      (`/Game/GAME/Framework/BP_Menu_Controller.Initial_Setup` _asbp_menu_controller))))

(event `UpdateLobby`
  (params (PlayerNames :type Boolean))
  (if PlayerNames
    (`KismetArrayLibrary.Array_Clear` (`self.ALL_PlayerProfiles`))
    (for _array_element (`self.AllConnectedPlayers`)
      (`KismetArrayLibrary.Array_Add` (`self.ALL_PlayerProfiles`) (`/Game/GAME/Framework/BP_Menu_Controller.Player ProfileInfo` _array_element)))
    (for _array_element_2 (`self.AllConnectedPlayers`)
      (if PlayerNames
        (`/Game/GAME/Framework/BP_Menu_Controller.UpdatePlayerNames` _array_element_2 (`self.ALL_PlayerProfiles`))))))

(fn `UserConstructionScript`)