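; Shooter game instance that handles the main and multiplayer menus, the player profile and game session flow.
; Showing the main menu loads the profile from a save slot, or creates a save object, and fills in the player name.
; Solo play opens the first level directly; multiplayer hosts a listen-server lobby with a LAN toggle or joins a session.
; Map changes run a servertravel console command.
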(event `StartSoloGame`
  (set `self.isSoloGame` true)
  (`GameplayStatics.OpenLevel` "FirstLevel"))

(event `ChangePlayerName`
  (params (PlayerName :type Text))
  (set `self.Player Profile_Info` (make `/Game/GAME/SaveData/S_PlayerProfile` PlayerName))
  (`self.SaveProfile`))

(event `CreateMultiSession`
  (set `self.isSoloGame` false)
  (`CreateSessionCallbackProxy.CreateSession` (`GameplayStatics.GetPlayerController` 0) 4 (`self.isLANConnection`)
    (:`OnSuccess`
      (`GameplayStatics.OpenLevel` "LobbyLevel" true "listen"))
    (:`OnFailure`
      (`KismetSystemLibrary.PrintString` "Faild to create Session"))))

(event `JoinMultiSession`
  (params (SessionResult :type "BlueprintSessionResult Structure"))
  (set `self.isSoloGame` false)
  (`JoinSessionCallbackProxy.JoinSession` (`GameplayStatics.GetPlayerController` 0) SessionResult
    (:`OnFailure`
      (`KismetSystemLibrary.PrintString` "Faild to join Session"))))

(event `TravelToMap`
  (params (NumOfPlayers :type Integer) (MapName :type String))
  (set `self.Num Of Players` NumOfPlayers)
  (`KismetSystemLibrary.ExecuteConsoleCommand` (`KismetStringLibrary.Concat_StrStr` "servertravel " MapName) (`GameplayStatics.GetPlayerController` 0)))

(fn `ChangeConnectionType`
  (returns (isLANGame :type Boolean))
  (bind _islanconnection (`self.isLANConnection`))
  (if _islanconnection
    (set `self.isLANConnection` false)
    (else
      (set `self.isLANConnection` true)))
  (return _islanconnection))

(fn `CheckForSaveProfile`
  (bind _returnvalue (`GameplayStatics.DoesSaveGameExist` (`self.PlayerProfile_Slot`)))
  (if _returnvalue
    (bind _asbp_save_player (`self.LoadProfile`))
    (set `self.Player Save Profile` _asbp_save_player)
    (else
      (`self.SaveProfile`)))
  (return))

(fn `LoadProfile`
  (returns (`AsBP Save Player` :type "/Game/GAME/SaveData/BP_SavePlayer Object Reference"))
  (bind _returnvalue (`GameplayStatics.LoadGameFromSlot` (`self.PlayerProfile_Slot`)))
  (bind _asbp_save_player (cast `/Game/GAME/SaveData/BP_SavePlayer` _returnvalue))
  (set `self.Player Profile_Info` (`/Game/GAME/SaveData/BP_SavePlayer.PlayerProfile` _asbp_save_player))
  (return _asbp_save_player))

(fn `SaveProfile`
  (bind _player_save_profile (`self.Player Save Profile`))
  (`/Engine/EditorBlueprintResources/StandardMacros.IsValid` (`self.Player Save Profile`)
    (:`Is Valid`
      (set `/Game/GAME/SaveData/BP_SavePlayer.PlayerProfile` (`self.Player Profile_Info`) _player_save_profile)
      (`GameplayStatics.SaveGameToSlot` _player_save_profile (`self.PlayerProfile_Slot`))
      (return))
    (:`Is Not Valid`
      (bind _returnvalue (`GameplayStatics.CreateSaveGameObject` "/Game/GAME/SaveData/BP_SavePlayer.BP_SavePlayer_C"))
      (set `self.Player Save Profile` _returnvalue))))

(fn `UI_ShowMainMenu`
  (bind _returnvalue (`GameplayStatics.GetPlayerController` 0))
  (`/Engine/EditorBlueprintResources/StandardMacros.IsValid` (`self.MainMenu BP`)
    (:`Is Valid`
      _)
    (:`Is Not Valid`
      (bind _returnvalue_2 (`|CreateWidget` "/Game/GAME/Widgets/Menu_Widgets/WB_MainMenu.WB_MainMenu_C" _returnvalue))
      (set `self.MainMenu BP` _returnvalue_2)))
  (`UserWidget.AddToViewport` (`self.MainMenu BP`) 0)
  (`WidgetBlueprintLibrary.SetInputMode_UIOnlyEx` _returnvalue null)
  (set `PlayerController.bShowMouseCursor` true _returnvalue)
  (`self.CheckForSaveProfile`)
  (`EditableText.SetText` (`/Game/GAME/Widgets/Menu_Widgets/WB_MainMenu.Input_PlayerName` (`self.MainMenu BP`)) (`.PlayerName_3_BB63628F438026FB979FDA8E46C14B1C` (break `/Game/GAME/SaveData/S_PlayerProfile` (`self.Player Profile_Info`))))
  (return))

(fn `UI_ShowMultiMenu`
  (`/Engine/EditorBlueprintResources/StandardMacros.IsValid` (`self.MultiMenu BP`)
    (:`Is Valid`
      _)
    (:`Is Not Valid`
      (bind _returnvalue (`|CreateWidget` "/Game/GAME/Widgets/Menu_Widgets/WB_MultiMenu.WB_MultiMenu_C" (`GameplayStatics.GetPlayerController` 0)))
      (set `self.MultiMenu BP` _returnvalue)))
  (`UserWidget.AddToViewport` (`self.MultiMenu BP`) 0)
  (return))