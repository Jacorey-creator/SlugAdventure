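; BP_Inventory is the player's backpack inventory, keeping a list of item strings on its owner.
; Adding appends and prints the item, while removing drops the first entry containing the given substring.
; Both operations cast the owner to BP_Player_AJ and update its BackpackWidget, with removal notifying the UI even without a match.
; Despite its name, InventoryEmpty returns true when the inventory has items.
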(fn `AddItemToInventory`
  (params (`New Item` :type String))
  (`KismetArrayLibrary.Array_Add` (`self.Inventory`) `New Item`)
  (`KismetSystemLibrary.PrintString` `New Item`)
  (bind _asbp_player_aj (cast `/Game/GAME/Characters/BP_Player_AJ` (`self.GetOwner`)))
  (`/Game/GAME/Widgets/User_Interface/WB_Backpack.ItemToBackPackUI` (`/Game/GAME/Characters/BP_Player_AJ.Backpack_Widget` _asbp_player_aj) `New Item`))

(fn `InventoryEmpty?`
  (returns (ContainsItem :type Boolean))
  (return (`KismetArrayLibrary.Array_IsNotEmpty` (`self.Inventory`))))

(fn `RemoveItemFromInventory`
  (params (`Item String` :type String))
  (for (_array_element _array_index) (`self.Inventory`)
    (if (`KismetStringLibrary.Contains` _array_element `Item String`)
      (`KismetArrayLibrary.Array_Remove` (`self.Inventory`) _array_index)
      (break)))
  (bind _asbp_player_aj (cast `/Game/GAME/Characters/BP_Player_AJ` (`self.GetOwner`)))
  (`/Game/GAME/Widgets/User_Interface/WB_Backpack.ItemOutOfBackPackUI` (`/Game/GAME/Characters/BP_Player_AJ.Backpack_Widget` _asbp_player_aj) `Item String`))