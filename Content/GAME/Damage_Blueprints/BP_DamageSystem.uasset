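; BP_DamageSystem is a reusable health and damage Blueprint that tracks health, death and invincibility.
; TakeDamage takes a DamageInfo struct and uses CanBeDamaged to ignore hits when dead, or when invincible unless the hit bypasses invincibility.
; Applied damage fires either the OnDeath or OnDamageResponse dispatcher and returns whether the hit landed.
; Heal restores health up to MaxHealth while alive.
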(fn `Heal`
  (params (Amount :type "Float (double-precision)"))
  (returns (`New Health` :type "Float (double-precision)"))
  (if (not (`self.isDead?`))
    (bind _output_get (set `self.Health` (`KismetMathLibrary.FClamp` (+ Amount (`self.Health`)) 0.0 (`self.Max_Health`))))
    (return _output_get)))

(fn `TakeDamage`
  (params (DamageInfo :type "/Game/GAME/Damage_Blueprints/S_DamageInfo Structure"))
  (returns (`WasDamaged?` :type Boolean))
  (bind (_damageamount _damagetype _damageresponse _damageinvincible_) (break `/Game/GAME/Damage_Blueprints/S_DamageInfo` DamageInfo))
  (`self.CanBeDamaged` _damageinvincible_
    (:`Do Damage`
      (bind _output_get (set `self.Health` (- (`self.Health`) _damageamount)))
      (if (<= _output_get 0.0)
        (set `self.isDead?` true)
        (`self.OnDeath`)
        (else
          (`self.OnDamageResponse` _damageresponse)))
      (return true))
    (:`Ignore Damage`
      (return false))))