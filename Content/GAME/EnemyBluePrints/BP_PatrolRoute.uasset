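; BP_PatrolRoute is a spline-based patrol path actor that tracks a current waypoint, likely for enemy patrols.
; IncrementPatrolRoute steps the point index by a direction value, which flips at the last and first spline points to produce a back-and-forth ping-pong route.
; GetSplinePointPosition returns the world-space location of the current point on the SRoute spline.
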(event `IncrementPatrolRoute`
  (bind _output_get (set `self.IndexPatrolPoint` (+ (`self.IndexPatrolPoint`) (`self.Direction`))))
  (if (== _output_get (- (`SplineComponent.GetNumberOfSplinePoints` (`self.S_Route`)) 1))
    (set `self.Direction` -1)
    (elif (== (`self.IndexPatrolPoint`) 0)
      (set `self.Direction` 1))))

(fn `GetSplinePointPosition`
  (returns (Location :type "Vector Structure"))
  (return (`SplineComponent.GetLocationAtSplinePoint` (`self.S_Route`) (`self.IndexPatrolPoint`) "World")))

(fn `UserConstructionScript`)