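; Ricochet variant of the slug projectile, which sets its slug type and ignores its owner when moving.
; On hit it reports the impact, increments the bounce count, then chains debug-drawn line traces along mirrored surface normals, up to the bounce limit.
; Successful traces call TransformSlug while bounces remain; the traces never redirect the projectile's movement.
; The construction script randomizes initial speed and applies max speed and gravity.
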(event `self.ReceiveBeginPlay`
  (set `self.Slug_Type` "NewEnumerator1")
  (`PrimitiveComponent.IgnoreActorWhenMoving` (`self.SphereCollision`) (`self.GetOwner`) true))

(event `self.ReceiveTick`
  (params (DeltaSeconds :type "Float (single-precision)"))
  (`parent.ReceiveTick` DeltaSeconds))

(event `self.SphereCollision.OnComponentHit`
  (params (HitComponent :type "PrimitiveComponent Object Reference") (OtherActor :type "Actor Object Reference") (OtherComp :type "PrimitiveComponent Object Reference") (NormalImpulse :type "Vector Structure") (Hit :type "HitResult Structure (by ref)"))
  (bind (_bblockinghit _binitialoverlap _time _distance _location _impactpoint _normal _impactnormal _physmat _hitactor _hitcomponent _hitbonename _bonename _hititem _elementindex _faceindex _tracestart _traceend) (`GameplayStatics.BreakHitResult` Hit))
  (bind _returnvalue (`KismetMathLibrary.MirrorVectorByNormal` (`KismetMathLibrary.GetDirectionUnitVector` _tracestart _traceend) _impactnormal))
  (bind _output_get (set `self.Hit` Hit))
  (`self.OnProjectileImpact` OtherActor _output_get)
  (bind _result (`/Engine/EditorBlueprintResources/StandardMacros.IncrementInt` (`self.Current_Bounces`))
    (:`  `
      (set `self.Current_Bounces` _result)
      (for _ (range (+ (`self.Max_Bounces`) 1))
        (if _bblockinghit
          (bind (_outhit _returnvalue_2) (`KismetSystemLibrary.LineTraceSingle` :`Start` (+ _impactpoint _returnvalue) :`End` (+ _impactpoint (* _returnvalue 100000.0)) :`TraceChannel` "TraceTypeQuery1" :`DrawDebugType` "ForDuration" :`DrawTime` 0.1))
          (set `self.Hit` _outhit)
          (if _returnvalue_2
            (if (>= (`self.Current_Bounces`) (`self.Max_Bounces`))
              (break)
              (else
                (`self.Transform Slug` (`self.Slug_Location`))))
            (else
              (break))))))))

(fn `UserConstructionScript`
  (bind _projectilemovement (`self.ProjectileMovement`))
  (set `ProjectileMovementComponent.InitialSpeed` (`KismetMathLibrary.RandomFloatInRange` (`self.MinSpeed`) (`self.Speed`)) _projectilemovement)
  (set `ProjectileMovementComponent.MaxSpeed` (`self.Speed`) _projectilemovement)
  (set `ProjectileMovementComponent.ProjectileGravityScale` (`self.Gravity`) _projectilemovement))