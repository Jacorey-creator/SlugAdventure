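; Ghoul variant of the slug projectile, built on a parent class that supplies its construction logic.
; On BeginPlay it sets its slug type, makes its collision sphere ignore the owning actor when moving, and rotates toward its target if one is valid.
; Overlap and Tick events are disabled stubs, so this graph adds only that startup setup.
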(event `self.ReceiveBeginPlay`
  (set `self.Slug_Type` "NewEnumerator3")
  (`PrimitiveComponent.IgnoreActorWhenMoving` (`self.SphereCollision`) (`self.GetOwner`) true)
  (`self.Target`
    (:`then`
      (`self.RotateToTarget`))
    (:`else`)))

(fn `UserConstructionScript`
  (`parent.UserConstructionScript`))