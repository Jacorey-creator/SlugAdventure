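; BP_GhoulSlug is a short-lived slug character that chases the player and is destroyed a few seconds after BeginPlay through its life span.
; The FollowPlayer event applies the slug's move speed, stores a player reference and runs AI MoveTo targeting the player character.
; Each successful move calls FollowPlayer again to continue the chase, with no handling for failure.
; Nothing in this graph makes the initial FollowPlayer call.
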(event `self.ReceiveBeginPlay`
  (`parent.ReceiveBeginPlay`)
  (`self.SetLifeSpan` 3.0))

(event `self.ReceiveTick`
  (params (DeltaSeconds :type "Float (single-precision)"))
  (`parent.ReceiveTick` DeltaSeconds))

(event `self.Follow Player`
  (bind _returnvalue (`GameplayStatics.GetPlayerCharacter` 0))
  (set `CharacterMovementComponent.MaxWalkSpeed` (`self.Slug_MoveSpeed`) (`self.CharacterMovement`))
  (set `self.Player REF` _returnvalue)
  (`|AIMoveTo` self (`self.PlayerPOS`) _returnvalue 0.0
    (:`OnSuccess`
      (`self.Follow Player`))))

(fn `UserConstructionScript`
  (`parent.UserConstructionScript`))