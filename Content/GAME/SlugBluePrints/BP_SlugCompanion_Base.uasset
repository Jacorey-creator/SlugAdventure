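; Base slug companion character that follows the player and reacts to contact according to its slug type.
; A self-repeating AIMoveTo trails the player at SlugMoveSpeed, while Tick caches the player's location.
; On capsule hits with BP_Player_AJ, Ricochet and Test slugs destroy themselves, while Ghoul slugs deal damage, then spark and vanish if it lands.
; PickUpItem shows a pickup popup widget and returns the Item.
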(event `self.ReceiveBeginPlay`
  (set `self.Slug_MoveSpeed` (`self.Slug_MoveSpeed`))
  (`self.Follow Player`))

(event `Follow Player`
  (bind _returnvalue (`GameplayStatics.GetPlayerCharacter` 0))
  (set `CharacterMovementComponent.MaxWalkSpeed` (`self.Slug_MoveSpeed`) (`self.CharacterMovement`))
  (set `self.Player REF` _returnvalue)
  (`|AIMoveTo` self (`self.PlayerPOS`) _returnvalue 275.0
    (:`OnSuccess`
      (`self.Follow Player`))))

(event `self.ReceiveTick`
  (params (DeltaSeconds :type "Float (single-precision)"))
  (`self.Get Player Position`))

(event `Get Player Position`
  (set `self.PlayerPOS` (`self.K2_GetActorLocation` (`self.Player REF`))))

(event `self.CapsuleComponent.OnComponentHit`
  (params (HitComponent :type "PrimitiveComponent Object Reference") (OtherActor :type "Actor Object Reference") (OtherComp :type "PrimitiveComponent Object Reference") (NormalImpulse :type "Vector Structure") (Hit :type "HitResult Structure (by ref)"))
  (bind _asbp_player_aj (cast `/Game/GAME/Characters/BP_Player_AJ` OtherActor))
  (switch `/Game/GAME/Characters/E_ListOfSlugs` (`self.Slug_Type`)
    (:`NewEnumerator1`
      (`self.K2_DestroyActor` :!label _label))
    (:`NewEnumerator2`
      (goto _label))
    (:`NewEnumerator3`
      (bind _wasdamaged (`/Game/GAME/Damage_Blueprints/BP_Damagable.TakeDamage` _asbp_player_aj (make `/Game/GAME/Damage_Blueprints/S_DamageInfo` 5.0 "NewEnumerator1")))
      (if _wasdamaged
        (`GameplayStatics.SpawnEmitterAtLocation` "/Game/StarterContent/Particles/P_Sparks.P_Sparks")
        (goto _label)))))

(fn `Pick Up Item`
  (returns (Item :type String))
  (bind _returnvalue (`|CreateWidget` "/Game/GAME/Widgets/User_Interface/WB_PickUpPopUp.WB_PickUpPopUp_C" (`GameplayStatics.GetPlayerController` 0)))
  (`UserWidget.AddToViewport` _returnvalue 0)
  (return (`self.Item`)))

(fn `UserConstructionScript`)