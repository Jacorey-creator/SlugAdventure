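; Base slug projectile that flies at a set speed and gravity, then turns into a slug actor on impact.
; Construction configures projectile movement, with optional homing on Target; BeginPlay ignores the owner in collision and aims velocity at any valid Target.
; On hit it reports the impact, then TransformSlug spawns the class matching SlugType just above the last ticked location and destroys the projectile.
; BeginPlay always sets SlugType to Test.
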(event `self.ReceiveBeginPlay`
  (set `self.Slug_Type` "NewEnumerator2")
  (`PrimitiveComponent.IgnoreActorWhenMoving` (`self.SphereCollision`) (`self.GetOwner`) true)
  (`self.Target`
    (:`then`
      (`self.RotateToTarget`))
    (:`else`)))

(event `RotateToTarget`
  (set `MovementComponent.Velocity` (* (`KismetMathLibrary.GetDirectionUnitVector` (`self.K2_GetActorLocation`) (`self.K2_GetActorLocation` (`self.Target`))) (`self.Speed`)) (`self.ProjectileMovement`)))

(event `self.ReceiveTick`
  (params (DeltaSeconds :type "Float (single-precision)"))
  (set `self.Slug_Location` (`self.K2_GetActorLocation`)))

(event `self.SphereCollision.OnComponentHit`
  (params (HitComponent :type "PrimitiveComponent Object Reference") (OtherActor :type "Actor Object Reference") (OtherComp :type "PrimitiveComponent Object Reference") (NormalImpulse :type "Vector Structure") (Hit :type "HitResult Structure (by ref)"))
  (`self.OnProjectileImpact` OtherActor Hit)
  (`self.Transform Slug` (`self.Slug_Location`)))

(fn `Transform Slug`
  (params (`Slug Location` :type "Vector Structure"))
  (bind _returnvalue (`KismetMathLibrary.Conv_VectorToTransform` (`KismetMathLibrary.MakeVector` `Slug Location_X` `Slug Location_Y` (+ `Slug Location_Z` 2.0))))
  (switch `/Game/GAME/Characters/E_ListOfSlugs` (`self.Slug_Type`)
    (:`NewEnumerator1`
      (`|SpawnActorFromClass` "/Game/GAME/SlugBluePrints/BP_SlugCompanion_Ricochet.BP_SlugCompanion_Ricochet_C" _returnvalue "Undefined" "MultiplyWithRoot" null null)
      (`self.K2_DestroyActor` self))
    (:`NewEnumerator2`
      (`|SpawnActorFromClass` "/Game/GAME/SlugBluePrints/BP_SlugCompanion_Base.BP_SlugCompanion_Base_C" _returnvalue "AdjustIfPossibleButAlwaysSpawn" "MultiplyWithRoot" null null)
      (`self.K2_DestroyActor` self))
    (:`NewEnumerator3`
      (`|SpawnActorFromClass` "/Game/GAME/SlugBluePrints/BP_GhoulSlug.BP_GhoulSlug_C" _returnvalue "AdjustIfPossibleButAlwaysSpawn" "MultiplyWithRoot" null null)
      (`self.K2_DestroyActor` self))))

(fn `UserConstructionScript`
  (bind _projectilemovement (`self.ProjectileMovement`))
  (set `ProjectileMovementComponent.InitialSpeed` (`self.Speed`) _projectilemovement)
  (set `ProjectileMovementComponent.MaxSpeed` (`self.Speed`) _projectilemovement)
  (set `ProjectileMovementComponent.ProjectileGravityScale` (`self.Gravity`) _projectilemovement)
  (`self.Target`
    (:`then`
      (if (`self.isHoming?`)
        (set `ProjectileMovementComponent.bIsHomingProjectile` true _projectilemovement)
        (set `ProjectileMovementComponent.HomingTargetComponent` (`Actor.RootComponent` (`self.Target`)) _projectilemovement)))
    (:`else`)))