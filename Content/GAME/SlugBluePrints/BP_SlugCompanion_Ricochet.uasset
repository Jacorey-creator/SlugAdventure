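; Ricochet variant of a slug companion actor that the player can pick up in the world.
; A capsule hit from BP_Player_AJ destroys the slug when its SlugType is Ricochet Slug or Test.
; Pick Up Item shows a WB_PickUpPopUp widget and returns the Item.
; BeginPlay, Tick and construction defer to the parent, and the nodes setting SelectedSlugClass to projectile classes are unconnected.
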(event `self.ReceiveBeginPlay`
  (`parent.ReceiveBeginPlay`))

(event `self.ReceiveActorBeginOverlap`
  (params (OtherActor :type "Actor Object Reference")))

(event `self.ReceiveTick`
  (params (DeltaSeconds :type "Float (single-precision)"))
  (`parent.ReceiveTick` DeltaSeconds))

(event `self.CapsuleComponent.OnComponentHit`
  (params (HitComponent :type "PrimitiveComponent Object Reference") (OtherActor :type "Actor Object Reference") (OtherComp :type "PrimitiveComponent Object Reference") (NormalImpulse :type "Vector Structure") (Hit :type "HitResult Structure (by ref)"))
  (cast `/Game/GAME/Characters/BP_Player_AJ` OtherActor)
  (switch `/Game/GAME/Characters/E_ListOfSlugs` (`self.Slug_Type`)
    (:`NewEnumerator1`
      _)
    (:`NewEnumerator2`
      _))
  (`self.K2_DestroyActor`))

(fn `Pick Up Item`
  (returns (Item :type String))
  (bind _returnvalue (`|CreateWidget` "/Game/GAME/Widgets/User_Interface/WB_PickUpPopUp.WB_PickUpPopUp_C" (`GameplayStatics.GetPlayerController` 0)))
  (`UserWidget.AddToViewport` _returnvalue 0)
  (return (`self.Item`)))

(fn `UserConstructionScript`
  (`parent.UserConstructionScript`))