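; Enemy character that patrols, punches and fires ghoul slug projectiles at the player, exposing actions, speed and patrol route for AI logic.
; BPDamageSystem handles health, feeding a widget health bar and triggering ragdoll death before destruction.
; Montage-driven attacks and gun draw fire end dispatchers on completion or interruption.
; Shots spawn after the montage ends, turning toward the tracked player location, with damage applied through a projectile impact binding.
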(event `self.ReceiveBeginPlay`
  (bind _returnvalue (`|CreateWidget` "/Game/GAME/Widgets/User_Interface/WB_HealthBar.WB_HealthBar_C" null self))
  (`WidgetComponent.SetWidget` (`self.Widget`) _returnvalue)
  (`BlackboardComponent.SetValueAsFloat` (`AIBlueprintHelperLibrary.GetBlackboard` null) "Range" (`self.Range`)))

(event `self.ReceiveTick`
  (params (DeltaSeconds :type "Float (single-precision)"))
  (bind _returnvalue (`GameplayStatics.GetPlayerCharacter` 0))
  (`/Engine/EditorBlueprintResources/StandardMacros.IsValid` _returnvalue
    (:`Is Valid`
      (set `self.Player Location` (`SceneComponent.K2_GetComponentLocation` (`Character.CapsuleComponent` _returnvalue))))))

(event `Damage Response`
  (params (`Damage Response` :type "/Game/GAME/Damage_Blueprints/E_Damage_Response Enum" :default "NewEnumerator0"))
  (`KismetSystemLibrary.PrintString` (`|GetEnumeratorNameAsString` `Damage Response`)))

(event `Death Event`
  (bind _mesh (`self.Mesh`))
  (`PrimitiveComponent.SetSimulatePhysics` _mesh true)
  (`PrimitiveComponent.SetCollisionEnabled` _mesh "QueryAndPhysics")
  (`KismetSystemLibrary.PrintString` "Dead")
  (`KismetSystemLibrary.Delay` 5.0)
  (`self.K2_DestroyActor`))

(event `FireWeapon`
  (`|PlayMontage` (`self.Mesh`) "/Game/GAME/Characters/Animations/Enemy/Attack/Shooting_Montage.Shooting_Montage"
    (:`OnCompleted`
      _)
    (:`OnInterrupted`
      _))
  (`self.OnFireEnd`)
  (bind _aim_direction (`self.AimAtPlayer`))
  (`self.K2_SetActorRotation` _aim_direction)
  (bind _returnvalue (`|SpawnActorFromClass` "/Game/GAME/SlugBluePrints/BP_SlugProjectile_Ghoul.BP_SlugProjectile_Ghoul_C" (`SceneComponent.K2_GetComponentToWorld` (`self.Arrow1`)) "Undefined" "MultiplyWithRoot" self 2000.0 1.0 null false null))
  (`PrimitiveComponent.IgnoreActorWhenMoving` (`self.CapsuleComponent`) _returnvalue true)
  (add `/Game/GAME/SlugBluePrints/BP_SlugProjectile_Base.OnProjectileImpact` _returnvalue (delegate `Damage Enemy`)))

(event `Damage Enemy`
  (params (`Other Actor` :type "Actor Object Reference") (Hit :type "HitResult Structure"))
  (bind (_bblockinghit _binitialoverlap _time _distance _location _impactpoint _normal _impactnormal _physmat _hitactor) (`GameplayStatics.BreakHitResult` Hit))
  (if (not (== `Other Actor` self))
    ;[1 1 1] Deal Damage
    (bind _wasdamaged (message `/Game/GAME/Damage_Blueprints/BP_Damagable.TakeDamage` _hitactor (make `/Game/GAME/Damage_Blueprints/S_DamageInfo` 10.0 "NewEnumerator2")))
    (`AISense_Damage.ReportDamageEvent` _hitactor self 10.0 (`self.K2_GetActorLocation`))
    (if _wasdamaged
      (`GameplayStatics.SpawnEmitterAtLocation` "/Game/StarterContent/Particles/P_Sparks.P_Sparks" _location))))

(event `PunchAttack`
  (`|PlayMontage` (`self.Mesh`) "/Game/GAME/Characters/Animations/Enemy/Attack/Punching_Montage.Punching_Montage"
    (:`OnCompleted`
      _)
    (:`OnInterrupted`
      _))
  (`self.OnAttackEnd`))

(event `WieldGun`
  (`|PlayMontage` (`self.Mesh`) "/Game/GAME/Characters/Animations/Enemy/Attack/Draw_Weapon_Montage.Draw_Weapon_Montage"
    (:`then`
      (`KismetSystemLibrary.Delay` 0.7)
      (`SceneComponent.ToggleVisibility` (`self.WeaponMesh`) false)
      (set `self.isWieldingGun` true))
    (:`OnCompleted`
      (`self.OnGunDrawnEnd` :!label _label))
    (:`OnInterrupted`
      (goto _label))))

(fn `AimAtPlayer`
  (returns (`Aim Direction` :type "Rotator Structure"))
  (`KismetSystemLibrary.LineTraceSingle` :`Start` (`SceneComponent.K2_GetComponentLocation` (`self.ProjectileSpawn Location`)) :`End` (`self.Player Location`) :`TraceChannel` "TraceTypeQuery1" :`DrawDebugType` "ForDuration")
  (return (`KismetMathLibrary.FindRelativeLookAtRotation` (`KismetMathLibrary.Conv_VectorToTransform` (`self.K2_GetActorLocation`)) (`self.Player Location`))))

(fn `Chambered_Slug`
  (if (not (not (>= (`self.SelectedSlug_Index`) (`KismetArrayLibrary.Array_Length` (`/Game/GAME/Backpack/BP_Inventory.Inventory` (`self.BP_Inventory`))))))
    (set `self.SelectedSlug_Index` 0))
  (bind _enumvalue (foreach `/Game/GAME/Characters/E_ListOfSlugs` false)
    (:`LoopBody`
      (bind _output_get (set `self.Slug_Name` (`|GetArrayItem` (`/Game/GAME/Backpack/BP_Inventory.Inventory` (`self.BP_Inventory`)) (`self.SelectedSlug_Index`))))
      (if (`KismetStringLibrary.Contains` _output_get (`|GetEnumeratorNameAsString` _enumvalue))
        (switch `/Game/GAME/Characters/E_ListOfSlugs` _enumvalue
          (:`NewEnumerator1`
            (set `self.SelectedSlugClass` "/Game/GAME/SlugBluePrints/BP_SlugProjectile_Ricochet.BP_SlugProjectile_Ricochet_C"))
          (:`NewEnumerator2`
            (set `self.SelectedSlugClass` "/Game/GAME/SlugBluePrints/BP_SlugProjectile_Base.BP_SlugProjectile_Base_C")))
        (return)))))

(fn `Get Attack Target`
  (returns (Target :type "Actor Object Reference"))
  (return null))

(fn `Get Patrol Route`
  (returns (PatrolRoute :type "/Game/GAME/EnemyBluePrints/BP_PatrolRoute Object Reference"))
  (return (`self.PatrolRoute`)))

(fn `GetCurrentHealth`
  (returns (Health :type "Float (double-precision)"))
  (return (`/Game/GAME/Damage_Blueprints/BP_DamageSystem.Health` (`self.BP_DamageSystem`))))

(fn `GetMaxHealth`
  (returns (`Max Health` :type "Float (double-precision)"))
  (return (`/Game/GAME/Damage_Blueprints/BP_DamageSystem.Max_Health` (`self.BP_DamageSystem`))))

(fn `Heal`
  (params (`Heal Amount` :type "Float (double-precision)"))
  (returns (`New Health` :type "Float (double-precision)"))
  (bind _new_health (`/Game/GAME/Damage_Blueprints/BP_DamageSystem.Heal` (`self.BP_DamageSystem`) `Heal Amount`))
  (return _new_health))

(fn `Random_Slug_Sound`
  (bind _asbp_shooter_gamemode (cast `/Game/GAME/Framework/BP_Shooter_Gamemode` (`GameplayStatics.GetGameMode`)))
  (bind _slug_sounds (`/Game/GAME/Framework/BP_Shooter_Gamemode.Slug_Sounds` _asbp_shooter_gamemode))
  (`GameplayStatics.PlaySound2D` (`|GetArrayItem` _slug_sounds (`KismetMathLibrary.RandomIntegerInRange` 0 (- (`KismetArrayLibrary.Array_Length` _slug_sounds) 1))) 1.0 1.0 0.0 null null)
  (return))

(fn `Set Movement Speed`
  (params (Speed :type "/Game/GAME/EnemyBluePrints/Enumerations/E_EnemySpeeds Enum" :default "NewEnumerator0"))
  (returns (SpeedValue :type "Float (double-precision)"))
  (bind _output_get (set `CharacterMovementComponent.MaxWalkSpeed` (select `/Game/GAME/EnemyBluePrints/Enumerations/E_EnemySpeeds` Speed :`NewEnumerator1` 250.0 :`NewEnumerator2` 500.0 :!type "Float (single-precision)") (`self.CharacterMovement`)))
  (return _output_get))

(fn `TakeDamage`
  (params (DamageInfo :type "/Game/GAME/Damage_Blueprints/S_DamageInfo Structure"))
  (returns (WasDamaged :type Boolean))
  (bind _wasdamaged_ (`/Game/GAME/Damage_Blueprints/BP_DamageSystem.TakeDamage` (`self.BP_DamageSystem`) DamageInfo))
  (return _wasdamaged_))

(fn `UserConstructionScript`
  (bind _bp_damagesystem (`self.BP_DamageSystem`))
  (add `/Game/GAME/Damage_Blueprints/BP_DamageSystem.OnDeath` _bp_damagesystem (`|CreateDelegate` :!event `Death Event`))
  (add `/Game/GAME/Damage_Blueprints/BP_DamageSystem.OnDamageResponse` _bp_damagesystem (`|CreateDelegate` :!event `Damage Response`))
  (`SceneComponent.ToggleVisibility` (`self.WeaponMesh`) false)
  (set `self.isWieldingGun` false))