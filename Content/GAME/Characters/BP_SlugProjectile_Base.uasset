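; BP_SlugProjectile_Base is a slug projectile that turns into a slug companion when it hits something.
; A hit on its Sphere component passes the impact location to TransformSlug, which switches on SlugType.
; The only handled type, Test, spawns BP_SlugCompanion_Base at that location and destroys the projectile.
; Tick also records the Sphere's world location in SlugLocation.
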(event `self.ReceiveBeginPlay`)

(event `self.ReceiveTick`
  (params (DeltaSeconds :type "Float (single-precision)"))
  (set `self.Slug_Location` (`SceneComponent.K2_GetComponentLocation` (`self.Sphere`))))

(event `self.Sphere.OnComponentHit`
  (params (HitComponent :type "PrimitiveComponent Object Reference") (OtherActor :type "Actor Object Reference") (OtherComp :type "PrimitiveComponent Object Reference") (NormalImpulse :type "Vector Structure") (Hit :type "HitResult Structure (by ref)"))
  (`self.TransformSlug` (`KismetMathLibrary.Conv_VectorToTransform` (`.Location` (`GameplayStatics.BreakHitResult` Hit)))))

(fn `TransformSlug`
  (params (SlugSpawnLocator :type "Transform Structure"))
  (switch `/Game/GAME/Characters/E_ListOfSlugs` (`self.Slug_Type`)
    (:`NewEnumerator2`
      (`|SpawnActorFromClass` "/Game/GAME/Characters/BP_SlugCompanion_Base.BP_SlugCompanion_Base_C" SlugSpawnLocator "Undefined" "MultiplyWithRoot" null null)
      (`self.K2_DestroyActor` self))))

(fn `UserConstructionScript`)