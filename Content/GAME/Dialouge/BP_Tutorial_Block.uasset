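; Tutorial zone actor that puts the player into tutorial mode and presents dialogue from the character Pronto.
; Box overlap by BP_Player_AJ hides the weapon mesh and sets the player's Tutorial flag.
; Each Talk event increments the index and shows that Dialouge entry in a lazily created WB_TutorialBox widget.
; Once the index exceeds the array length, it shows a repeat quip, waits, resets and calls Talk again.
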(event `self.Box.OnComponentBeginOverlap`
  (params (OverlappedComponent :type "PrimitiveComponent Object Reference") (OtherActor :type "Actor Object Reference") (OtherComp :type "PrimitiveComponent Object Reference") (OtherBodyIndex :type Integer) (bFromSweep :type Boolean) (SweepResult :type "HitResult Structure (by ref)"))
  (bind _asbp_player_aj (cast `/Game/GAME/Characters/BP_Player_AJ` OtherActor))
  (`SceneComponent.SetVisibility` (`/Game/GAME/Characters/BP_Player_AJ.WeaponMesh` _asbp_player_aj) false false)
  (set `/Game/GAME/Characters/BP_Player_AJ.Tutorial?` true _asbp_player_aj))

(event `/Game/GAME/Dialouge/BPI_Dialouge.Talk`
  (`/Engine/EditorBlueprintResources/StandardMacros.IncrementInt` (`self.TalkIndex`)
    (:`  `
      (if (<= (`self.TalkIndex`) (`KismetArrayLibrary.Array_Length` (`self.Dialouge`)))
        (`self.UI`
          (:`then`
            _)
          (:`else`
            (bind _returnvalue (`|CreateWidget` "/Game/GAME/Widgets/Tutorial/WB_TutorialBox.WB_TutorialBox_C" (`GameplayStatics.GetPlayerController` 0)))
            (bind _output_get (set `self.UI` _returnvalue))
            (`UserWidget.AddToViewport` _output_get 0)))
        (`TextBlock.SetText` (`/Game/GAME/Widgets/Tutorial/WB_TutorialBox.Tutorial_Text` (`self.UI`)) (`KismetTextLibrary.Conv_StringToText` (`|GetArrayItem` (`self.Dialouge`) (`self.TalkIndex`))))
        (else
          (`TextBlock.SetText` (`/Game/GAME/Widgets/Tutorial/WB_TutorialBox.Tutorial_Text` (`self.UI`)) "Ah, lost in the labyrinth of your own mind, I see! Fear not, for Pronto shall repeat himself with unmatched grace! Ahem...")
          (`KismetSystemLibrary.Delay` 3.0)
          (set `self.TalkIndex` 0)
          (`self.Talk`))))))

(fn `UserConstructionScript`)